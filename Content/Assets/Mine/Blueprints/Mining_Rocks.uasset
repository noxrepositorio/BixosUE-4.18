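; Clickable mining rock for a top-down game that starts a quick-time event and grants an inventory reward.
; A click starts a looping timer that waits for the player to enter the capsule, then stops movement and runs QTE.
; QTE opens the pickaxe widget's puzzle at the rock's screen position, or warns when no pickaxes remain.
; Sucesso adds the prize, destroying the rock if everything fits.
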(event OnClicked(StaticMesh)
  (params (TouchedComponent :type Primitive%20Component%20Object%20Reference) (ButtonPressed :type Key%20Structure))
  (bind _returnvalue (Utilities|Time|SetTimerbyEvent (delegate Custom|WaitChartoQTE) 0.2 true))
  (Variables|Default|SetWaitCharHandle _returnvalue))

(event OnBeginCursorOver(StaticMesh)
  (params (TouchedComponent :type Primitive%20Component%20Object%20Reference))
  (Variables|/Script/Engine.PlayerController|SetCurrentMouseCursor (Game|GetPlayerController 0) "Hand"))

(event OnEndCursorOver(StaticMesh)
  (params (TouchedComponent :type Primitive%20Component%20Object%20Reference))
  (Variables|/Script/Engine.PlayerController|SetCurrentMouseCursor (Game|GetPlayerController 0) "Default"))

(event OnComponentBeginOverlap(Capsule)
  (params (OverlappedComponent :type Primitive%20Component%20Object%20Reference) (OtherActor :type Actor%20Object%20Reference) (OtherComp :type Primitive%20Component%20Object%20Reference) (OtherBodyIndex :type Integer) (bFromSweep :type Boolean) (SweepResult :type Hit%20Result%20Structure%20%28by%20ref%29))
  (bind _astop_down_character (Utilities|Casting|CastToTopDownCharacter (Game|GetPlayerCharacter 0)))
  (if (== OtherActor _astop_down_character)
    (Variables|Default|SetCharInCapsule true)
    (Components|Movement|StopMovementImmediately (Variables|/Script/Engine.Character|GetCharacterMovement _astop_down_character))))

(event OnComponentEndOverlap(Capsule)
  (params (OverlappedComponent :type Primitive%20Component%20Object%20Reference) (OtherActor :type Actor%20Object%20Reference) (OtherComp :type Primitive%20Component%20Object%20Reference) (OtherBodyIndex :type Integer))
  (bind _astop_down_character (Utilities|Casting|CastToTopDownCharacter (Game|GetPlayerCharacter 0)))
  (if (== OtherActor _astop_down_character)
    (Variables|Default|SetCharInCapsule false)))

(event Custom|WaitChartoQTE
  (if (Variables|Default|GetCharInCapsule)
    (CallFunction|QTE)
    (Utilities|Time|ClearandInvalidateTimerbyHandle (Variables|Default|GetWaitCharHandle))
    (bind _astop_down_character (Utilities|Casting|CastToTopDownCharacter (Game|GetPlayerCharacter 0)))
    (Components|Movement|StopMovementImmediately (Variables|/Script/Engine.Character|GetCharacterMovement _astop_down_character))))

(fn ConstructionScript)

(fn QTE
  (bind _returnvalue (Game|GetPlayerController 0))
  (bind _defaultsceneroot (Variables|Default|GetDefaultSceneRoot))
  (bind _returnvalue_2 (Transformation|GetWorldLocation _defaultsceneroot))
  (bind _screenposition (Class|GameplayStatics|ProjectWorldtoScreen _returnvalue _returnvalue_2 true))
  (bind _foundwidgets (Widget|GetAllWidgetsOfClass "/Game/TopDownBP/Widgets/Mining_pickaxe_UI.Mining_pickaxe_UI_C" true))
  (if (> (Variables|/Game/TopDownBP/Widgets/Mining_pickaxe_UI.Mining_pickaxe_UI_C|GetPickaxeAmount (Utilities|Array|Get(acopy) _foundwidgets)) 0)
    (Variables|/Game/TopDownBP/Widgets/Mining_pickaxe_UI.Mining_pickaxe_UI_C|SetRock_ref (Utilities|Array|Get(acopy) _foundwidgets) self)
    (Default|StartQTE (Utilities|Array|Get(acopy) _foundwidgets) "NewEnumerator0" (.x _screenposition) (.y _screenposition))
    (else
      (bind _astop_down_controller (Utilities|Casting|CastToTopDownController (Game|GetPlayerController 0)))
      (Default|CaixaDeMensagem _astop_down_controller true false false false "" "Você necessita de picaretas para minerar!" "Ok"))))

(fn Sucesso
  (bind _astop_down_game_mode (Utilities|Casting|CastToTopDownGameMode (Game|GetGameMode)))
  (bind (_sucess_ _rest_) (Default|AddItem (Variables|/Game/TopDownBP/Blueprints/TopDownGameMode.TopDownGameMode_C|GetInventario%20Ref _astop_down_game_mode) (Variables|Default|GetPremio) (Variables|Default|GetQuantidadePremio)))
  (if _sucess_
    (if (not (> _rest_ 0))
      (Actor|DestroyActor))))